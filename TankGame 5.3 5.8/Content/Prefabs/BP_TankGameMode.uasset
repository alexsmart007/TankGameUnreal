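; BP_TankGameMode is the tank game's game mode, handling HUD feedback and background music.
; On BeginPlay it creates the WBP_HUD widget and starts a 2D music track.
; Level-start and lives events update the HUD, while level-complete, win and game-over events show messages and stop the music.
; Only the win and game-over messages show buttons; the file contains no logic that decides these outcomes.
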(event EventBeginPlay
  (bind _returnvalue (UserInterface|CreateWidget "/Game/Prefabs/WBP_HUD.WBP_HUD_C" (Game|GetPlayerController 0)))
  (bind _output_get (Variables|Default|SetHUD _returnvalue))
  (UserInterface|Viewport|AddtoViewport _output_get 0)
  (bind _returnvalue_2 (Audio|SpawnSound2D "/Game/Audio/053_-_Tanks_-_Variation_1.053_-_Tanks_-_Variation_1" 0.5 1.0 0.0 0))
  (Variables|Default|SetMusic _returnvalue_2))

(event EventTick
  (params (DeltaSeconds :type Float%20%28single-precision%29)))

(event EventOnLivesChanged
  (params (Lives :type Integer))
  (Default|SetLives (Variables|Default|GetHUD) Lives))

(event EventOnLevelStarted
  (params (Level :type Integer))
  (Default|SetLevel (Variables|Default|GetHUD) Level))

(event EventOnLevelComplete
  (params (Level :type Integer))
  (Default|ShowMessage (Variables|Default|GetHUD) (Utilities|Text|FormatText "Level {0} Complete!" Level) false)
  (Audio|Components|Audio|Stop (Variables|Default|GetMusic)))

(event EventOnGameOver
  (Default|ShowMessage (Variables|Default|GetHUD) "Game Over" true)
  (Audio|Components|Audio|Stop (Variables|Default|GetMusic)))

(event EventOnWin
  (Default|ShowMessage (Variables|Default|GetHUD) "You Win!" true)
  (Audio|Components|Audio|Stop (Variables|Default|GetMusic)))

(fn ConstructionScript)